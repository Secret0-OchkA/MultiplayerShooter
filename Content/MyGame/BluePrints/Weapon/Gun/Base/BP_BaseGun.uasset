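; Base gun Blueprint that fires projectile actors in single, auto or burst mode through fire start and stop interface events.
; An EndShot flag, delays and a gate pace the shots, while CaclulateAmmo handles magazine spend, reload and reserve changes.
; Each bullet's transform aims from the muzzle toward a trace from the shooter's camera location along the owner's forward vector, with random rotational spread.
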(event EventIFireStop
  ;[1 1 1] auto fire
  (Utilities|FlowControl|Gate true) ; enters at Close
)

(event EventIFireStart
  (switch Utilities|FlowControl|Switch|SwitchonENUM_FireType "NewEnumerator0"
    (:NewEnumerator0
      ;[1 1 1] single
      (if (and (> (Variables|WeaponStats|Ammo|Magazin|GetAmmoMagazinCurrent) 0) (Variables|Default|GetendShot))
        (Variables|Default|SetendShot false)
        (CallFunction|FireBullet)
        (CallFunction|CaclulateAmmo "NewEnumerator0")
        (Utilities|FlowControl|Delay 0.0)
        (Variables|Default|SetendShot true)
        (Development|PrintString (Utilities|String|Append (Utilities|String|ToString(Integer) (Variables|WeaponStats|Ammo|Magazin|GetAmmoMagazinCurrent)) "/" (Utilities|String|ToString(Integer) (Variables|WeaponStats|Ammo|GetAmmoCurrent))) true true "(R=0.000000,G=1.000000,B=0.022722,A=1.000000)")))
    (:NewEnumerator1
      ;[1 1 1] auto fire
      (Utilities|FlowControl|Sequence
        (:then_0
          (if (Variables|Default|GetendShot)
            (goto _label Open)))
        (:then_1
          (Utilities|FlowControl|Gate true :!label _label
            (:Exit
              (Variables|Default|SetendShot false)
              (if (> (Variables|WeaponStats|Ammo|Magazin|GetAmmoMagazinCurrent) 0)
                (CallFunction|FireBullet)
                (CallFunction|CaclulateAmmo "NewEnumerator0")
                (Utilities|FlowControl|Delay 1.0)
                (Variables|Default|SetendShot true)
                (goto _label)
                (else
                  (goto _label Close))))))))
    (:NewEnumerator2
      ;[1 1 1] Burst
      (if (Variables|Default|GetendShot)
        (if (and (> (Variables|WeaponStats|Ammo|Magazin|GetAmmoMagazinCurrent) 0) (< (Variables|Default|GetCurrentBurstShot) (Variables|WeaponStats|GetBurstBullet))) :!label _label_2
          (Variables|Default|SetendShot false)
          (CallFunction|FireBullet)
          (CallFunction|CaclulateAmmo "NewEnumerator0")
          (Utilities|FlowControl|Delay 0.2)
          (Variables|Default|SetCurrentBurstShot (+ (Variables|Default|GetCurrentBurstShot) 1))
          (goto _label_2)
          (else
            (Variables|Default|SetCurrentBurstShot 0)
            (Variables|Default|SetendShot true)))))))

(fn ConstructionScript
  (Variables|WeaponStats|Ammo|Magazin|SetAmmoMagazinCurrent (Variables|WeaponStats|Ammo|Magazin|GetAmmoMagazinMax))
  (Variables|WeaponStats|Ammo|SetAmmoCurrent (Variables|WeaponStats|Ammo|GetAmmoMax)))

(fn Calculate
  (bind _muzzleposition (Utilities|MuzzlePosition))
  (bind _asbp_shooter_charecter (Utilities|Casting|CastToBP_ShooterCharecter (Game|GetInstigator)))
  (bind (_outhit _returnvalue) (Collision|LineTraceForObjects (Transformation|GetWorldLocation (Variables|/Game/MyGame/BluePrints/Charecter/BP_ShooterCharecter.BP_ShooterCharecter_C|GetCamera _asbp_shooter_charecter)) (+ (Transformation|GetWorldLocation (Variables|/Game/MyGame/BluePrints/Charecter/BP_ShooterCharecter.BP_ShooterCharecter_C|GetCamera _asbp_shooter_charecter)) (* (Transformation|GetActorForwardVector (Components|GetOwner)) 1e+04)) (Utilities|Array|MakeArray "ObjectTypeQuery1") false 0 "ForDuration"))
  (return _muzzleposition (Math|Rotator|FindLookatRotation _muzzleposition (Math|Vector|SelectVector (.ImpactPoint (Collision|BreakHitResult _outhit)) (+ (Transformation|GetWorldLocation (Variables|/Game/MyGame/BluePrints/Charecter/BP_ShooterCharecter.BP_ShooterCharecter_C|GetCamera _asbp_shooter_charecter)) (* (Transformation|GetActorForwardVector (Components|GetOwner)) 1e+04)) _returnvalue))))

(fn CalculateFinal
  (params (NewParam :type Vector) (A :type Rotator))
  (bind _spread (Variables|WeaponStats|GetSpread))
  (bind _returnvalue (* _spread -1.0))
  (return (Math|Transform|MakeTransform NewParam (Math|Rotator|CombineRotators A (Math|Rotator|MakeRotator (Math|Random|RandomFloatinRange _returnvalue _spread) (Math|Random|RandomFloatinRange _returnvalue _spread) (Math|Random|RandomFloatinRange _returnvalue _spread))))))

(fn CalculateDirection
  (bind (_location _rotation) (Direction|Calculate))
  (bind _transform (Direction|CalculateFinal _location _rotation))
  (return _transform))

(fn CaclulateAmmo
  (params (Action :type ENUM_CalculateAmmo%20Enum :default "NewEnumerator0") (AddAmmo :type Integer))
  (switch Utilities|FlowControl|Switch|SwitchonENUM_CalculateAmmo Action
    (:NewEnumerator0
      ;[1 1 1] Fire
      (if (> (Variables|WeaponStats|Ammo|Magazin|GetAmmoMagazinCurrent) 0)
        (Variables|WeaponStats|Ammo|Magazin|SetAmmoMagazinCurrent (- (Variables|WeaponStats|Ammo|Magazin|GetAmmoMagazinCurrent) 1))))
    (:NewEnumerator2
      ;[1 1 1] Reload
      (LocalVariables|SetDeltaMagazinAmmo (- (Variables|WeaponStats|Ammo|Magazin|GetAmmoMagazinMax) (Variables|WeaponStats|Ammo|Magazin|GetAmmoMagazinCurrent)))
      (if (<= (LocalVariables|GetDeltaMagazinAmmo) (Variables|WeaponStats|Ammo|GetAmmoCurrent))
        (Variables|WeaponStats|Ammo|Magazin|SetAmmoMagazinCurrent (Variables|WeaponStats|Ammo|Magazin|GetAmmoMagazinMax))
        (Variables|WeaponStats|Ammo|SetAmmoCurrent (- (Variables|WeaponStats|Ammo|GetAmmoCurrent) (LocalVariables|GetDeltaMagazinAmmo)))
        (else
          (Variables|WeaponStats|Ammo|Magazin|SetAmmoMagazinCurrent (+ (Variables|WeaponStats|Ammo|Magazin|GetAmmoMagazinCurrent) (Variables|WeaponStats|Ammo|GetAmmoCurrent)))
          (Variables|WeaponStats|Ammo|SetAmmoCurrent 0))))
    (:NewEnumerator1
      ;[1 1 1] AddAmmo
      (if (< (Variables|WeaponStats|Ammo|GetAmmoCurrent) (Variables|WeaponStats|Ammo|GetAmmoMax))
        (if (<= (- (Variables|WeaponStats|Ammo|GetAmmoCurrent) AddAmmo) (Variables|WeaponStats|Ammo|GetAmmoMax))
          (Variables|WeaponStats|Ammo|SetAmmoCurrent (- (Variables|WeaponStats|Ammo|GetAmmoCurrent) AddAmmo))
          (else
            (Variables|WeaponStats|Ammo|SetAmmoCurrent (Variables|WeaponStats|Ammo|GetAmmoMax)))))))
  (return (Variables|WeaponStats|Ammo|Magazin|GetAmmoMagazinCurrent)))

(fn OnRepAmmoCurrent)

(fn OnRepAmmoMagazinCurrent)

(fn FireBullet
  (bind _projectiletransform (CallFunction|CalculateDirection))
  (Game|SpawnActorfromClass (Variables|Bullet|GetBullet_Class) _projectiletransform "Undefined" (Components|GetOwner) (Game|GetInstigator)))