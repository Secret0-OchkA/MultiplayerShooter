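; Health component that tracks a current health value, applies damage and handles optional automatic regeneration.
; ChangeHealth is the shared entry point: it adds a delta, clamps between zero and Max, and calls Dead at zero, which only prints a message.
; Damage subtracts health, pauses regeneration and sets a delay timer.
; Tick then regenerates at a frame-rate-independent speed while enabled, below Max and not paused.
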(event Custom|Event%20StartRegeneration
  (Variables|Regeneration|Private|SetStartReg true))

(event EventBeginPlay
  (Variables|Health|SetCurrent (Variables|Health|GetMax)))

(event EventTick
  (params (DeltaSeconds :type Float%20%28single-precision%29))
  (CallFunction|Regeneration))

(fn ChangeHealth
  (params (DeltaHealth :type Float%20%28single-precision%29))
  (Variables|Health|SetCurrent (+ DeltaHealth (Variables|Health|GetCurrent)))
  (|if(Current>Max)Current=Max)
  (|If(Curretn<0)Current=0)
  (if (<= (Variables|Health|GetCurrent) 0.0)
    (CallFunction|Dead)))

(fn Regeneration
  (if (Math|Boolean|ANDBoolean (Variables|Regeneration|GetOff/On) (< (Variables|Health|GetCurrent) (Variables|Health|GetMax)) (Variables|Regeneration|Private|GetStartReg))
    (CallFunction|ChangeHealth (* (Variables|Regeneration|GetSpeed) (Utilities|Time|GetWorldDeltaSeconds)))))

(fn Dead
  (Development|PrintString "dead"))

(fn Damage
  (params (A :type Float%20%28single-precision%29))
  (CallFunction|ChangeHealth (* A -1.0))
  (Utilities|Time|SetTimerbyEvent (EventDispatchers|CreateEvent :!event Custom|Event%20StartRegeneration) (Variables|Regeneration|GetDelay))
  (Variables|Regeneration|Private|SetStartReg false))