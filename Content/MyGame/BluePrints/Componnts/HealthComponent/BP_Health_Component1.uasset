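; Health component that tracks current health, starting at max, and handles damage and healing through IDamage and IHealing events.
; Both events feed ChangeHealth, which clamps the value between zero and max and calls Dead at zero, currently just a debug print.
; Damage pauses regeneration and sets a delay timer to resume it; Tick then restores health at a frame-rate-independent speed while enabled and below max.
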(event Custom|Event%20StartRegeneration
  (Variables|Regeneration|Private|SetStartReg true))

(event EventBeginPlay
  (Variables|Health|SetCurrent (Variables|Health|GetMax)))

(event EventTick
  (params (DeltaSeconds :type Float%20%28single-precision%29))
  (CallFunction|Regeneration))

(event EventIDamage
  (params (Damage :type Float%20%28single-precision%29))
  ;[1 1 1] Damage
  (Development|PrintString "Hello" true true "(R=1.000000,G=0.194613,B=0.000000,A=1.000000)")
  (CallFunction|ChangeHealth (* Damage -1.0))
  (Utilities|Time|SetTimerbyEvent (EventDispatchers|CreateEvent :!event Custom|Event%20StartRegeneration) (Variables|Regeneration|GetDelay))
  (Variables|Regeneration|Private|SetStartReg false))

(event EventIHealing
  (params (Health :type Float%20%28single-precision%29))
  ;[1 1 1] Healing
  (CallFunction|ChangeHealth Health))

(fn ChangeHealth
  (params (DeltaHealth :type Float%20%28single-precision%29))
  (Variables|Health|SetCurrent (+ DeltaHealth (Variables|Health|GetCurrent)))
  (|if(Current>Max)Current=Max)
  (|If(Curretn<0)Current=0)
  (if (<= (Variables|Health|GetCurrent) 0.0)
    (CallFunction|Dead)))

(fn Regeneration
  (if (Math|Boolean|ANDBoolean (Variables|Regeneration|GetOff/On) (< (Variables|Health|GetCurrent) (Variables|Health|GetMax)) (Variables|Regeneration|Private|GetStartReg))
    (CallFunction|ChangeHealth (* (Variables|Regeneration|GetSpeed) (Utilities|Time|GetWorldDeltaSeconds))))
  (return))

(fn Dead
  (Development|PrintString "dead"))

(fn OnRepCurrent)